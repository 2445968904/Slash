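; Left pipe-slide actor that repositions the player along a spline on overlapping its collision while Sprinting, or Standing with Wallmod.
; If a short forward trace from the spline start is clear, timelines turn the character to the spline's rotation and drive capsule movement.
; The move lerp uses TargetLocation for both ends, and the PipeSlide state change is disconnected.
; Leaving the collision restores Standing after a delay.
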(event `self.DetectCollision.OnComponentBeginOverlap`
  (params (OverlappedComponent :type "PrimitiveComponent Object Reference") (OtherActor :type "Actor Object Reference") (OtherComp :type "PrimitiveComponent Object Reference") (OtherBodyIndex :type Integer) (bFromSweep :type Boolean) (SweepResult :type "HitResult Structure (by ref)"))
  (bind (_character_nm _character_lpsp _camera _character) (`/Game/Code/NaturalMovementV3/Blueprint/NMFunctionLibrary/BP_NMFunctionLibrary.NMCharacter`))
  (bind _returnvalue (`SplineComponent.GetLocationAtSplinePoint` (`self.Spline`) 0 "World"))
  ;[1 0 0.0652] Pipe Slide Logic
  (if (== OtherActor (`.Character` (`/Game/Code/NaturalMovementV3/Blueprint/NMFunctionLibrary/BP_NMFunctionLibrary.NMCharacter`)))
    (switch `/Game/Code/NaturalMovementV3/Blueprint/Enum/Enum_MovementStates` (`/Game/Code/NaturalMovementV3/Blueprint/NMFunctionLibrary/BP_NMFunctionLibrary.States`)
      (:`NewEnumerator4`
        (bind (_outhit _returnvalue_2) (`KismetSystemLibrary.LineTraceSingle` :`Start` _returnvalue :`End` (+ (* (`SceneComponent.GetForwardVector` (`/Game/Code/NaturalMovementV3/Blueprint/NMFunctionLibrary/BP_NMFunctionLibrary.NMCapsuleComponent`)) 100.0) _returnvalue) :`TraceChannel` "TraceTypeQuery2" :`bIgnoreSelf` false :!label _label))
        (if (not _returnvalue_2)
          (`|ExecutionSequence`
            (:`then_0`
              (set `self.CurrentRotation` (`self.K2_GetActorRotation` _character))
              (bind (_direction `_新建轨道_0`) (`Timeline|Timeline_0` :!via `PlayFromStart`)
                (:`Update`
                  (bind _returnvalue_3 (`KismetMathLibrary.RLerp` (`self.CurrentRotation`) (`SplineComponent.GetRotationAtSplinePoint` (`self.Spline`) 2 "World") `_新建轨道_0` true))
                  (`self.K2_SetActorRotation` _character _returnvalue_3 false)
                  (`KismetSystemLibrary.PrintString` (`KismetStringLibrary.Conv_RotatorToString` _returnvalue_3)))))
            (:`then_1`
              (`self.TimeMove` (`SplineComponent.GetLocationAtSplinePoint` (`self.Spline`) 1 "World"))
              (`self.TimeMove` (`SplineComponent.GetLocationAtSplinePoint` (`self.Spline`) 2 "World"))))))
      (:`NewEnumerator1`
        (if (`self.wallmod`)
          (goto _label))))))

(event `self.DetectCollision.OnComponentEndOverlap`
  (params (OverlappedComponent :type "PrimitiveComponent Object Reference") (OtherActor :type "Actor Object Reference") (OtherComp :type "PrimitiveComponent Object Reference") (OtherBodyIndex :type Integer))
  ;[1 0 0.0652] Pipe Slide Logic
  (if (== OtherActor (`.Character` (`/Game/Code/NaturalMovementV3/Blueprint/NMFunctionLibrary/BP_NMFunctionLibrary.NMCharacter`)))
    (`KismetSystemLibrary.Delay` 4.0)
    (`/Game/Code/NaturalMovementV3/Blueprint/NMFunctionLibrary/BP_NMFunctionLibrary.SetvarEnumPlayerState` "NewEnumerator1")))

(event `TimeMove`
  (params (TargetLocation :type "Vector Structure"))
  (bind _capsulecomponent (`/Game/Code/NaturalMovementV3/Blueprint/NMFunctionLibrary/BP_NMFunctionLibrary.NMCapsuleComponent`))
  (set `self.Target Location` (`SceneComponent.K2_GetComponentLocation` _capsulecomponent))
  (bind (_direction `_新建轨道_0`) (`Timeline|坐标` :!via `PlayFromStart`)
    (:`Update`
      (`SceneComponent.K2_SetWorldLocation` _capsulecomponent (`KismetMathLibrary.VLerp` (`self.Target Location`) TargetLocation `_新建轨道_0`) false false))))

(fn `UserConstructionScript`)