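; Water volume actor that drives player swimming, diving and drowning for both NM and LPSP characters.
; Tick compares first-person camera height to the water plane, switching on swimming near the surface and restoring walking when overlap ends.
; While swimming submerged, it blends in underwater post-process and drains stamina, applying delayed damage when low; surfacing restores stamina.
; Input is enabled only while swimming, letting a downward axis pitch the view and nudge the capsule under.
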(event `self.WaterCollision.OnComponentBeginOverlap`
  (params (OverlappedComponent :type "PrimitiveComponent Object Reference") (OtherActor :type "Actor Object Reference") (OtherComp :type "PrimitiveComponent Object Reference") (OtherBodyIndex :type Integer) (bFromSweep :type Boolean) (SweepResult :type "HitResult Structure (by ref)"))
  (bind (_character_nm _character_lpsp _camera _character _isnmcharacter) (`/Game/Code/NaturalMovementV3/Blueprint/NMFunctionLibrary/BP_NMFunctionLibrary.NMCharacter`))
  ;[1 0 0.0652] Update
  (if (== OtherActor _character)
    (if (`/Game/Code/NaturalMovementV3/Blueprint/NMFunctionLibrary/BP_NMFunctionLibrary.InState?` "NewEnumerator4")
      (if _isnmcharacter
        (set `/Game/Code/NaturalMovementV3/Blueprint/Character/BP_NMCharacter.varEnumPlayerState` "NewEnumerator1" _character_nm)
        (else
          (set `/Game/Code/GameMain/LowPolyShooterPack/Core/Characters/BP_LPSP_PCH.varEnumPlayerState` "NewEnumerator1" _character_lpsp))))))

(event `InputAxis|SwimmingDown`
  (params (AxisValue :type "Float (single-precision)"))
  (bind _capsulecomponent (`/Game/Code/NaturalMovementV3/Blueprint/NMFunctionLibrary/BP_NMFunctionLibrary.NMCapsuleComponent`))
  (bind (_character_nm _character_lpsp _camera _character) (`/Game/Code/NaturalMovementV3/Blueprint/NMFunctionLibrary/BP_NMFunctionLibrary.NMCharacter`))
  (bind (_returnvalue_x _returnvalue_y _returnvalue_z) (`KismetMathLibrary.BreakVector` (`SceneComponent.K2_GetComponentLocation` _capsulecomponent)))
  (bind (_returnvalue_x_2 _returnvalue_y_2 _returnvalue_z_2) (`KismetMathLibrary.BreakVector` (`SceneComponent.K2_GetComponentLocation` (`/Game/Code/NaturalMovementV3/Blueprint/NMFunctionLibrary/BP_NMFunctionLibrary.NMFPCamera`))))
  (bind (_returnvalue_x_3 _returnvalue_y_3 _returnvalue_z_3) (`KismetMathLibrary.BreakVector` (`SceneComponent.K2_GetComponentLocation` (`self.WaterPlane`))))
  (bind (_returnvalue_roll _returnvalue_pitch _returnvalue_yaw) (`KismetMathLibrary.BreakRotator` (`Pawn.GetControlRotation` _character)))
  ;[1 0 0.0652] Swimming Down
  (if (and (< AxisValue 0.0) (not (< _returnvalue_z_2 _returnvalue_z_3)))
    (`Controller.SetControlRotation` (`GameplayStatics.GetPlayerController` 0) (`KismetMathLibrary.RInterpTo` (`Pawn.GetControlRotation` _character) (`KismetMathLibrary.MakeRotator` _returnvalue_roll -70.0 _returnvalue_yaw) (`GameplayStatics.GetWorldDeltaSeconds`) 10.0))
    (`/Engine/EditorBlueprintResources/StandardMacros.DoOnce` false :!label _label
      (:`Completed`
        (`KismetSystemLibrary.MoveComponentTo` _capsulecomponent (`KismetMathLibrary.MakeVector` _returnvalue_x _returnvalue_y (+ _returnvalue_z -60.0)) (`SceneComponent.RelativeRotation` _capsulecomponent) true true 0.3)
        (goto _label :!via `Reset`)))))

(event `self.WaterCollision.OnComponentEndOverlap`
  (params (OverlappedComponent :type "PrimitiveComponent Object Reference") (OtherActor :type "Actor Object Reference") (OtherComp :type "PrimitiveComponent Object Reference") (OtherBodyIndex :type Integer))
  (bind _charactermovement (`/Game/Code/NaturalMovementV3/Blueprint/NMFunctionLibrary/BP_NMFunctionLibrary.NMCharacterMovement`))
  (bind (_character_nm _character_lpsp _camera _character _isnmcharacter) (`/Game/Code/NaturalMovementV3/Blueprint/NMFunctionLibrary/BP_NMFunctionLibrary.NMCharacter`))
  ;[1 0 0.0652] End Swim
  (if (== OtherActor (`.Character` (`/Game/Code/NaturalMovementV3/Blueprint/NMFunctionLibrary/BP_NMFunctionLibrary.NMCharacter`)))
    (set `PhysicsVolume.bWaterVolume` false (`MovementComponent.GetPhysicsVolume` _charactermovement))
    (`CharacterMovementComponent.SetMovementMode` _charactermovement "MOVE_Walking" 0)
    (if _isnmcharacter
      (set `/Game/Code/NaturalMovementV3/Blueprint/Character/BP_NMCharacter.varEnumPlayerState` "NewEnumerator1" _character_nm)
      (`/Game/Code/NaturalMovementV3/Blueprint/Character/BP_NMCharacter.Request: Reset Jump Do Once` _character_nm)
      (`/Game/Code/NaturalMovementV3/Blueprint/NMFunctionLibrary/BP_NMFunctionLibrary.InWater` false)
      (else
        (set `/Game/Code/GameMain/LowPolyShooterPack/Core/Characters/BP_LPSP_PCH.varEnumPlayerState` "NewEnumerator1" _character_lpsp)
        (`/Game/Code/GameMain/LowPolyShooterPack/Core/Characters/BP_LPSP_PCH.Request: Reset Jump Do Once` _character_lpsp)
        (`/Game/Code/NaturalMovementV3/Blueprint/NMFunctionLibrary/BP_NMFunctionLibrary.InWater` false)))))

(event `self.ReceiveTick`
  (params (DeltaSeconds :type "Float (single-precision)"))
  (bind (_character_nm _character_lpsp _camera _character _isnmcharacter) (`/Game/Code/NaturalMovementV3/Blueprint/NMFunctionLibrary/BP_NMFunctionLibrary.NMCharacter`))
  (bind (_character_nm_2 _character_lpsp_2 _camera_2 _character_2 _isnmcharacter_2) (`/Game/Code/NaturalMovementV3/Blueprint/NMFunctionLibrary/BP_NMFunctionLibrary.NMCharacter`))
  (bind _returnvalue (`GameplayStatics.GetPlayerController` 0))
  (bind _waterpp (`self.WaterPP`))
  (bind _waterpp_2 (`self.WaterPP`))
  (bind (_returnvalue_x _returnvalue_y _returnvalue_z) (`KismetMathLibrary.BreakVector` (`SceneComponent.K2_GetComponentLocation` (`/Game/Code/NaturalMovementV3/Blueprint/NMFunctionLibrary/BP_NMFunctionLibrary.NMFPCamera`))))
  (bind (_returnvalue_x_2 _returnvalue_y_2 _returnvalue_z_2) (`KismetMathLibrary.BreakVector` (`SceneComponent.K2_GetComponentLocation` (`self.WaterPlane`))))
  (bind (_returnvalue_x_3 _returnvalue_y_3 _returnvalue_z_3) (`KismetMathLibrary.BreakVector` (`SceneComponent.K2_GetComponentLocation` (`/Game/Code/NaturalMovementV3/Blueprint/NMFunctionLibrary/BP_NMFunctionLibrary.NMFPCamera`))))
  (bind (_returnvalue_x_4 _returnvalue_y_4 _returnvalue_z_4) (`KismetMathLibrary.BreakVector` (`SceneComponent.K2_GetComponentLocation` (`self.WaterPlane`))))
  (bind (_returnvalue_x_5 _returnvalue_y_5 _returnvalue_z_5) (`KismetMathLibrary.BreakVector` (`SceneComponent.K2_GetComponentLocation` (`/Game/Code/NaturalMovementV3/Blueprint/NMFunctionLibrary/BP_NMFunctionLibrary.NMFPCamera`))))
  (bind (_returnvalue_x_6 _returnvalue_y_6 _returnvalue_z_6) (`KismetMathLibrary.BreakVector` (`SceneComponent.K2_GetComponentLocation` (`self.WaterPlane`))))
  (bind _returnvalue_2 (`KismetMathLibrary.Vector_Distance` (`KismetMathLibrary.MakeVector` 0.0 0.0 _returnvalue_z_5) (`KismetMathLibrary.MakeVector` 0.0 0.0 _returnvalue_z_6)))
  (bind _returnvalue_3 (and (not (< _returnvalue_z_3 _returnvalue_z_4)) (`PrimitiveComponent.IsOverlappingActor` (`self.WaterCollision`) (`.Character` (`/Game/Code/NaturalMovementV3/Blueprint/NMFunctionLibrary/BP_NMFunctionLibrary.NMCharacter`)))))
  ;[1 0 0.0652] Swim Logic
  (`|ExecutionSequence`
    (:`then_0`
      (`|ExecutionSequence`
        (:`then_0`
          (if (and (< _returnvalue_z _returnvalue_z_2) (`PrimitiveComponent.IsOverlappingActor` (`self.WaterCollision`) (`.Character` (`/Game/Code/NaturalMovementV3/Blueprint/NMFunctionLibrary/BP_NMFunctionLibrary.NMCharacter`))))
            (`|ExecutionSequence`
              (:`then_0`
                (if (`/Game/Code/NaturalMovementV3/Blueprint/NMFunctionLibrary/BP_NMFunctionLibrary.InState?` "NewEnumerator5")
                  (`|ExecutionSequence`
                    (:`then_0`
                      (set `PostProcessComponent.BlendWeight` (`KismetMathLibrary.FInterpTo` (`PostProcessComponent.BlendWeight` _waterpp_2) 1.0 (`GameplayStatics.GetWorldDeltaSeconds`) 5.0) _waterpp_2)
                      (`/Game/Code/NaturalMovementV3/Blueprint/NMFunctionLibrary/BP_NMFunctionLibrary.Global Stamina` -5.0 1.0)
                      (if _isnmcharacter_2
                        (set `/Game/Code/NaturalMovementV3/Blueprint/Character/BP_NMCharacter.varMoveRightAcceleration` 1.0 _character_nm_2)
                        (else
                          (set `/Game/Code/GameMain/LowPolyShooterPack/Core/Characters/BP_LPSP_PCH.varMoveRightAcceleration` 1.0 _character_lpsp_2))))
                    (:`then_1`
                      (`/Engine/EditorBlueprintResources/StandardMacros.DoOnce` false :!label _label_2
                        (:`Completed`
                          (`/Game/Code/NaturalMovementV3/UI/Widgets/WBP_BeginScreen.Play Sprint Animation` (`/Game/Code/NaturalMovementV3/Blueprint/NMFunctionLibrary/BP_NMFunctionLibrary.NMBeginScreenWidget`))
                          (goto _label_3 :!via `Reset`)))))))
              (:`then_1`
                (if (<= (`/Game/Code/NaturalMovementV3/Blueprint/NMFunctionLibrary/BP_NMFunctionLibrary.NMStaminaRange`) 10.0)
                  (`KismetSystemLibrary.Delay` 1.5)
                  (if (not (`/Game/Code/NaturalMovementV3/Blueprint/NMFunctionLibrary/BP_NMFunctionLibrary.InWater?`))
                    (`GameplayStatics.ApplyDamage` (`.Character` (`/Game/Code/NaturalMovementV3/Blueprint/NMFunctionLibrary/BP_NMFunctionLibrary.NMCharacter`)) 20.0))))
              (:`then_2`
                (`/Game/Code/NaturalMovementV3/Blueprint/NMFunctionLibrary/BP_NMFunctionLibrary.InWater` false)))))
        (:`then_1`
          (if _returnvalue_3
            (set `PostProcessComponent.BlendWeight` (`KismetMathLibrary.FInterpTo` (`PostProcessComponent.BlendWeight` _waterpp) 0.0 (`GameplayStatics.GetWorldDeltaSeconds`) 5.0) _waterpp)
            (`|ExecutionSequence`
              (:`then_0`
                (`/Engine/EditorBlueprintResources/StandardMacros.DoOnce` false :!label _label_3
                  (:`Completed`
                    (`/Game/Code/NaturalMovementV3/UI/Widgets/WBP_BeginScreen.End Sprint Animation` (`/Game/Code/NaturalMovementV3/Blueprint/NMFunctionLibrary/BP_NMFunctionLibrary.NMBeginScreenWidget`))
                    (goto _label_2 :!via `Reset`))))
              (:`then_1`
                (`/Game/Code/NaturalMovementV3/Blueprint/NMFunctionLibrary/BP_NMFunctionLibrary.Global Stamina` 15.0 1.0)))))
        (:`then_2`
          (if _returnvalue_3
            (`|ExecutionSequence`
              (:`then_0`
                (if (and (> _returnvalue_2 0.0) (< _returnvalue_2 40.0))
                  (`/Game/Code/NaturalMovementV3/Blueprint/NMFunctionLibrary/BP_NMFunctionLibrary.InWater` true)
                  (`CharacterMovementComponent.SetMovementMode` (`/Game/Code/NaturalMovementV3/Blueprint/NMFunctionLibrary/BP_NMFunctionLibrary.NMCharacterMovement`) "MOVE_Swimming" 0)
                  (if _isnmcharacter
                    (set `/Game/Code/NaturalMovementV3/Blueprint/Character/BP_NMCharacter.varEnumPlayerState` "NewEnumerator5" _character_nm)
                    (set `PhysicsVolume.bWaterVolume` true (`MovementComponent.GetPhysicsVolume` (`/Game/Code/NaturalMovementV3/Blueprint/NMFunctionLibrary/BP_NMFunctionLibrary.NMCharacterMovement`)))
                    (else
                      (set `/Game/Code/GameMain/LowPolyShooterPack/Core/Characters/BP_LPSP_PCH.varEnumPlayerState` "NewEnumerator5" _character_lpsp)
                      (set `PhysicsVolume.bWaterVolume` true (`MovementComponent.GetPhysicsVolume` (`/Game/Code/NaturalMovementV3/Blueprint/NMFunctionLibrary/BP_NMFunctionLibrary.NMCharacterMovement`)))))))
              (:`then_1`
                (if (> _returnvalue_2 40.0)
                  (set `PhysicsVolume.bWaterVolume` false (`MovementComponent.GetPhysicsVolume` (`/Game/Code/NaturalMovementV3/Blueprint/NMFunctionLibrary/BP_NMFunctionLibrary.NMCharacterMovement`))))))))))
    (:`then_1`
      (if (`/Game/Code/NaturalMovementV3/Blueprint/NMFunctionLibrary/BP_NMFunctionLibrary.InState?` "NewEnumerator5")
        (`/Engine/EditorBlueprintResources/StandardMacros.DoOnce` false :!label _label_4
          (:`Completed`
            (`self.EnableInput` _returnvalue)
            (goto _label_5 :!via `Reset`)))
        (else
          (`/Engine/EditorBlueprintResources/StandardMacros.DoOnce` false :!label _label_5
            (:`Completed`
              (`self.DisableInput` _returnvalue)
              (`/Game/Code/NaturalMovementV3/UI/Widgets/WBP_BeginScreen.End Sprint Animation` (`/Game/Code/NaturalMovementV3/Blueprint/NMFunctionLibrary/BP_NMFunctionLibrary.NMBeginScreenWidget`))
              (goto _label_4 :!via `Reset`))))))))

(fn `UserConstructionScript`)