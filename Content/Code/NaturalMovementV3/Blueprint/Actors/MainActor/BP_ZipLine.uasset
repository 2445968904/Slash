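; Zipline actor that the player boards with JumpEnd inside its Interact overlap and rides from spline start to end.
; Boarding attaches the character to AttachPoint, then timed component moves carry Origin along while a timeline turns the view and plays shake and radial blur.
; Pressing JumpEnd again far enough from the start detaches and launches the rider.
; The construction script fits meshes to the spline, flagging extra points or an end set too high.
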(event `InputAction|JumpEnd`
  (params (Key :type "Key Structure"))
  (bind (_character_nm _character_lpsp _camera _character _isnmcharacter) (`/Game/Code/NaturalMovementV3/Blueprint/NMFunctionLibrary/BP_NMFunctionLibrary.NMCharacter`))
  ;[1 0 0.0652] Active Zipline
  ;;[1 0 0.0652] Space ""
  (:`Pressed`
    (`/Engine/EditorBlueprintResources/StandardMacros.Gate` true :!label _label
      (:`Exit`
        (`/Engine/EditorBlueprintResources/StandardMacros.DoOnce` false :!label _label_2
          (:`Completed`
            (`self.Request: Start ZipLine`)
            (if _isnmcharacter
              (set `/Game/Code/NaturalMovementV3/Blueprint/Character/BP_NMCharacter.varEnumPlayerState` "NewEnumerator17" _character_nm)
              (else
                (set `/Game/Code/GameMain/LowPolyShooterPack/Core/Characters/BP_LPSP_PCH.varEnumPlayerState` "NewEnumerator17" _character_lpsp)))
            (`/Game/Code/NaturalMovementV3/Blueprint/NMFunctionLibrary/BP_NMFunctionLibrary.ClampYaw`)
            (goto _label :!via `Close`)))))))

(event `self.Interact.OnComponentBeginOverlap`
  (params (OverlappedComponent :type "PrimitiveComponent Object Reference") (OtherActor :type "Actor Object Reference") (OtherComp :type "PrimitiveComponent Object Reference") (OtherBodyIndex :type Integer) (bFromSweep :type Boolean) (SweepResult :type "HitResult Structure (by ref)"))
  ;[1 0 0.0652] Active Zipline
  (if (== OtherActor (`.Character` (`/Game/Code/NaturalMovementV3/Blueprint/NMFunctionLibrary/BP_NMFunctionLibrary.NMCharacter`)))
    (`self.EnableInput` (`GameplayStatics.GetPlayerController` 0))
    (goto _label :!via `Open`)))

(event `self.Interact.OnComponentEndOverlap`
  (params (OverlappedComponent :type "PrimitiveComponent Object Reference") (OtherActor :type "Actor Object Reference") (OtherComp :type "PrimitiveComponent Object Reference") (OtherBodyIndex :type Integer))
  (bind (_character_nm _character_lpsp _camera _character) (`/Game/Code/NaturalMovementV3/Blueprint/NMFunctionLibrary/BP_NMFunctionLibrary.NMCharacter`))
  ;[1 0 0.0652] Active Zipline
  (if (== OtherActor _character)
    (if (`/Game/Code/NaturalMovementV3/Blueprint/NMFunctionLibrary/BP_NMFunctionLibrary.InState?` "NewEnumerator17")
      (goto _label_2 :!via `Reset`)
      (else
        (`self.DisableInput` (`GameplayStatics.GetPlayerController` 0))
        (set `/Game/Code/GameMain/LowPolyShooterPack/Core/Characters/BP_LPSP_PCH.InPipe` false _character_lpsp)))))

(event `Request: Start ZipLine`
  (bind _charactermovement (`/Game/Code/NaturalMovementV3/Blueprint/NMFunctionLibrary/BP_NMFunctionLibrary.NMCharacterMovement`))
  (bind (_character_nm _character_lpsp _camera _character) (`/Game/Code/NaturalMovementV3/Blueprint/NMFunctionLibrary/BP_NMFunctionLibrary.NMCharacter`))
  (bind _capsulecomponent (`/Game/Code/NaturalMovementV3/Blueprint/NMFunctionLibrary/BP_NMFunctionLibrary.NMCapsuleComponent`))
  (bind (_character_nm_2 _character_lpsp_2 _camera_2 _character_2 _isnmcharacter) (`/Game/Code/NaturalMovementV3/Blueprint/NMFunctionLibrary/BP_NMFunctionLibrary.NMCharacter`))
  (bind _zipline (`self.ZipLine`))
  ;[1 0 0.0652] Start ZipLine Movement
  (`/Game/Code/NaturalMovementV3/Blueprint/NMFunctionLibrary/BP_NMFunctionLibrary.PlayCameraShake` "/Game/Code/NaturalMovementV3/Blueprint/Misc/CameraShake/ZipLine/BP_ZipLineStartCameraShake.BP_ZipLineStartCameraShake_C" 1.0)
  (`/Game/Code/GameMain/LowPolyShooterPack/Core/Characters/BP_LPSP_PCH.On Run Released` _character_lpsp_2)
  (set `/Game/Code/GameMain/LowPolyShooterPack/Core/Characters/BP_LPSP_PCH.ZipLine` self _character_lpsp_2)
  (if _isnmcharacter
    (set `/Game/Code/NaturalMovementV3/Blueprint/Character/BP_NMCharacter.varEnumMovementInput` "NewEnumerator0" _character_nm_2)
    (set `/Game/Code/NaturalMovementV3/Blueprint/Character/BP_NMCharacter.varEnumMouseInput` "NewEnumerator1" _character_nm_2)
    (else
      (set `/Game/Code/GameMain/LowPolyShooterPack/Core/Characters/BP_LPSP_PCH.varEnumMovementInput` "NewEnumerator0" _character_lpsp_2)
      (set `/Game/Code/GameMain/LowPolyShooterPack/Core/Characters/BP_LPSP_PCH.varEnumMouseInput` "NewEnumerator1" _character_lpsp_2)))
  (set `CharacterMovementComponent.GravityScale` 0.0 _charactermovement)
  (set `MovementComponent.Velocity` (0.0 0.0 0.0) _charactermovement)
  (`KismetSystemLibrary.MoveComponentTo` _capsulecomponent (+ (* (`SceneComponent.GetUpVector` _capsulecomponent) -90.0) (`SplineComponent.GetLocationAtSplinePoint` (`self.ZipLine`) 0 "World")) (`SceneComponent.RelativeRotation` _capsulecomponent) false false 0.5 :!label _label_3)
  (`|ExecutionSequence`
    (:`then_0`
      (`self.K2_AttachToComponent` (`.Character` (`/Game/Code/NaturalMovementV3/Blueprint/NMFunctionLibrary/BP_NMFunctionLibrary.NMCharacter`)) (`self.AttachPoint`) "None" "KeepWorld" "KeepRelative" "SnapToTarget" true)
      (`KismetSystemLibrary.MoveComponentTo` (`self.Origin`) (`self.varEndLocation`) (`SceneComponent.RelativeRotation` (`self.Origin`)) false false (`self.Time`) :!label _label_4)
      (`SceneComponent.K2_DetachFromComponent` (`/Game/Code/NaturalMovementV3/Blueprint/NMFunctionLibrary/BP_NMFunctionLibrary.NMCapsuleComponent`) "KeepWorld" "KeepWorld" "KeepWorld" true :!label _label_5)
      (set `CharacterMovementComponent.GravityScale` 1.0 (`/Game/Code/NaturalMovementV3/Blueprint/NMFunctionLibrary/BP_NMFunctionLibrary.NMCharacterMovement`))
      (`/Game/Code/NaturalMovementV3/Blueprint/NMFunctionLibrary/BP_NMFunctionLibrary.PlayCameraShake` "/Game/Code/NaturalMovementV3/Blueprint/Misc/CameraShake/ZipLine/BP_ZipLineEndCameraShake.BP_ZipLineEndCameraShake_C" 1.0)
      (`SceneComponent.K2_SetRelativeLocation` (`self.Origin`) (0.0 0.0 0.0) false false)
      (`/Game/Code/NaturalMovementV3/Blueprint/NMFunctionLibrary/BP_NMFunctionLibrary.Enable Movement`)
      (`self.DisableInput` (`GameplayStatics.GetPlayerController` 0)))
    (:`then_1`
      (`TimelineComponent.SetTimelineLength` (`self.RotationTime`) (`self.Time`))
      (`Timeline|RotationTime` :!via `PlayFromStart`
        (:`Update`
          (`/Game/Code/NaturalMovementV3/Blueprint/NMFunctionLibrary/BP_NMFunctionLibrary.PlayCameraShake` "/Game/Code/NaturalMovementV3/Blueprint/Misc/CameraShake/Parkour/Pipe/BP_PipeSlideDownCameraShake1.BP_PipeSlideDownCameraShake1_C" 0.5)
          (`/Game/Code/NaturalMovementV3/Blueprint/NMFunctionLibrary/BP_NMFunctionLibrary.RadialBlur` 0.3 1.0)
          (`Controller.SetControlRotation` (`GameplayStatics.GetPlayerController` 0) (`KismetMathLibrary.RInterpTo` (`Pawn.GetControlRotation` _character) (`KismetMathLibrary.FindLookAtRotation` (`self.K2_GetActorLocation` _character) (+ (* (`SceneComponent.GetUpVector` _zipline) -100.0) (`SplineComponent.GetLocationAtSplinePoint` _zipline 1 "World"))) (`GameplayStatics.GetWorldDeltaSeconds`) 3.0)))))))

(event `Quite_ZipLine`
  (bind (_character_nm _character_lpsp _camera _character _isnmcharacter) (`/Game/Code/NaturalMovementV3/Blueprint/NMFunctionLibrary/BP_NMFunctionLibrary.NMCharacter`))
  ;[1 0 0.0652] Start ZipLine Movement
  (if (`/Game/Code/NaturalMovementV3/Blueprint/NMFunctionLibrary/BP_NMFunctionLibrary.InState?` "NewEnumerator17") :!label _label_6
    (if (> (`KismetMathLibrary.Vector_Distance` (`SceneComponent.K2_GetComponentLocation` (`self.SM_ZipLine`)) (`self.K2_GetActorLocation` (`.Character` (`/Game/Code/NaturalMovementV3/Blueprint/NMFunctionLibrary/BP_NMFunctionLibrary.NMCharacter`)))) 600.0)
      (`|ExecutionSequence`
        (:`then_0`
          (goto _label_3 :!via `Stop`))
        (:`then_1`
          (goto _label_4 :!via `Stop`))
        (:`then_2`
          (goto _label_5))
        (:`then_3`
          (`Timeline|Launch Character` :!via `PlayFromStart`
            (:`Update`
              (if _isnmcharacter
                (`/Game/Code/NaturalMovementV3/Blueprint/Character/BP_NMCharacter.Request: To Jump End` _character_nm)
                (`self.DisableInput` (`GameplayStatics.GetPlayerController` 0))
                (else
                  (`/Game/Code/GameMain/LowPolyShooterPack/Core/Characters/BP_LPSP_PCH.Request: To Jump End` _character_lpsp)
                  (`self.DisableInput` (`GameplayStatics.GetPlayerController` 0)))))))))))

(event `InputAction|JumpEnd`
  (params (Key :type "Key Structure"))
  ;[1 0 0.0652] Start ZipLine Movement
  (:`Pressed`
    (goto _label_6)))

(fn `UserConstructionScript`
  (bind _bad (`self.Bad`))
  (bind _enddebug (`self.EndDebug`))
  (bind _zipline (`self.ZipLine`))
  (bind _bad_2 (`self.Bad`))
  (bind (_returnvalue_x _returnvalue_y _returnvalue_z) (`KismetMathLibrary.BreakVector` (`SplineComponent.GetLocationAtSplinePoint` (`self.ZipLine`) 0 "Local")))
  (bind (_relativelocation_x _relativelocation_y _relativelocation_z) (`KismetMathLibrary.BreakVector` (`SceneComponent.RelativeLocation` (`self.Bad`))))
  ;[1 0 0.0652] Zipline
  (`|ExecutionSequence`
    (:`then_0`
      (for _index (range (+ (- (`SplineComponent.GetNumberOfSplinePoints` _zipline) 2) 1))
        (bind _returnvalue (+ _index 1))
        (bind _location (`SplineComponent.GetLocationAndTangentAtSplinePoint` _zipline _returnvalue "Local"))
        (`SceneComponent.K2_SetRelativeLocation` (`self.Cable`) _location false false)
        (`|ExecutionSequence`
          (:`then_0`
            (set `self.varEndLocation` (`SplineComponent.GetLocationAndTangentAtSplinePoint` _zipline _returnvalue "Local"))
            (`SceneComponent.K2_SetRelativeLocation` _enddebug (+ _location (* (`SceneComponent.GetRightVector` _enddebug) 90.0)) false false)
            (`SceneComponent.K2_SetRelativeLocation` _bad (+ _location (* (`SceneComponent.GetUpVector` _bad) 40.0)) false false)
            (if (>= _returnvalue_z _relativelocation_z)
              (`SceneComponent.SetVisibility` _bad_2 false false)
              (else
                (`SceneComponent.SetVisibility` _bad_2 true false)
                (set `self.varBad` true))))
          (:`then_1`
            (bind (_returnvalue_roll _returnvalue_pitch _returnvalue_yaw) (`KismetMathLibrary.BreakRotator` (`KismetMathLibrary.FindLookAtRotation` (`SplineComponent.GetLocationAndTangentAtSplinePoint` _zipline _index "Local") _location)))
            (`SceneComponent.K2_SetRelativeRotation` (`self.SM_ZipLine`) (`KismetMathLibrary.MakeRotator` 0.0 0.0 _returnvalue_yaw) false false)
            (`SceneComponent.K2_SetRelativeRotation` (`self.Interact`) (`KismetMathLibrary.MakeRotator` 0.0 0.0 _returnvalue_yaw) false false)
            (`SceneComponent.K2_SetRelativeRotation` (`self.SM_ZipLine1`) (`KismetMathLibrary.MakeRotator` 0.0 0.0 _returnvalue_yaw) false false))
          (:`then_2`
            (`SceneComponent.K2_SetRelativeLocation` (`self.SM_ZipLine1`) _location false false)))))
    (:`then_1`
      (if (> (`SplineComponent.GetNumberOfSplinePoints` (`self.ZipLine`)) 2)
        (`SceneComponent.SetVisibility` (`self.Bad`) true false)
        (set `self.varBad` true)))))