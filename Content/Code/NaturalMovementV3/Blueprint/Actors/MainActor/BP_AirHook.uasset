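; BP_AirHook is an air hook point actor that starts the player character's hook.
; When its TraceCollision is overlapped by BP_LPSP_PCH, it prints a debug string and calls RequestBeginHook on that character, passing itself.
; Tick and the construction script are empty.
; Disconnected leftover logic covers a camera-trace hook crosshair, a hook reset request, and snapping the actor to a height above the ground.
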(event `self.ReceiveTick`
  (params (DeltaSeconds :type "Float (single-precision)"))
  ;[1 0 0.0652] Hook
)

(event `self.TraceCollision.OnComponentBeginOverlap`
  (params (OverlappedComponent :type "PrimitiveComponent Object Reference") (OtherActor :type "Actor Object Reference") (OtherComp :type "PrimitiveComponent Object Reference") (OtherBodyIndex :type Integer) (bFromSweep :type Boolean) (SweepResult :type "HitResult Structure (by ref)"))
  (bind _asbp_lpsp_pch (cast `/Game/Code/GameMain/LowPolyShooterPack/Core/Characters/BP_LPSP_PCH` OtherActor))
  (`KismetSystemLibrary.PrintString` "Trace")
  (`/Game/Code/GameMain/LowPolyShooterPack/Core/Characters/BP_LPSP_PCH.Request:Begin Hook` _asbp_lpsp_pch self))

(fn `UserConstructionScript`
  ;[1 0 0.0652] Set Default Offset
)