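; Interactive door actor that the player opens from either side by holding Interaction, or kicks through at speed.
; Two trigger volumes enable input and show a widget whose progress bar follows the hold timeline.
; A full hold swings the door via timeline while MoveComponentTo carries the movement-locked player through, then snaps it shut.
; Entering a trigger fast, grounded and passing a short line trace runs a quicker kick with camera animation.
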(event `self.ActiveDoorTrace_2.OnComponentBeginOverlap`
  (params (OverlappedComponent :type "PrimitiveComponent Object Reference") (OtherActor :type "Actor Object Reference") (OtherComp :type "PrimitiveComponent Object Reference") (OtherBodyIndex :type Integer) (bFromSweep :type Boolean) (SweepResult :type "HitResult Structure (by ref)"))
  (bind _capsulecomponent (`/Game/Code/NaturalMovementV3/Blueprint/NMFunctionLibrary/BP_NMFunctionLibrary.NMCapsuleComponent`))
  (bind _capsulecomponent_2 (`/Game/Code/NaturalMovementV3/Blueprint/NMFunctionLibrary/BP_NMFunctionLibrary.NMCapsuleComponent`))
  (bind _capsulecomponent_3 (`/Game/Code/NaturalMovementV3/Blueprint/NMFunctionLibrary/BP_NMFunctionLibrary.NMCapsuleComponent`))
  (bind _capsulecomponent_4 (`/Game/Code/NaturalMovementV3/Blueprint/NMFunctionLibrary/BP_NMFunctionLibrary.NMCapsuleComponent`))
  (bind _capsulecomponent_5 (`/Game/Code/NaturalMovementV3/Blueprint/NMFunctionLibrary/BP_NMFunctionLibrary.NMCapsuleComponent`))
  (bind (_character_nm _character_lpsp _camera _character _isnmcharacter) (`/Game/Code/NaturalMovementV3/Blueprint/NMFunctionLibrary/BP_NMFunctionLibrary.NMCharacter`))
  (bind (_returnvalue_x _returnvalue_y) (`KismetMathLibrary.BreakVector` (`SceneComponent.K2_GetComponentLocation` (`self.Go to Right Start`))))
  (bind (_returnvalue_x_2 _returnvalue_y_2 _returnvalue_z) (`KismetMathLibrary.BreakVector` (`SceneComponent.K2_GetComponentLocation` _capsulecomponent)))
  (bind (_returnvalue_x_3 _returnvalue_y_3) (`KismetMathLibrary.BreakVector` (`SceneComponent.K2_GetComponentLocation` (`self.Go to Right End`))))
  (bind (_returnvalue_x_4 _returnvalue_y_4 _returnvalue_z_2) (`KismetMathLibrary.BreakVector` (`SceneComponent.K2_GetComponentLocation` _capsulecomponent_2)))
  (bind (_returnvalue_x_5 _returnvalue_y_5) (`KismetMathLibrary.BreakVector` (`SceneComponent.K2_GetComponentLocation` (`self.Go to Left End`))))
  (bind (_returnvalue_x_6 _returnvalue_y_6 _returnvalue_z_3) (`KismetMathLibrary.BreakVector` (`SceneComponent.K2_GetComponentLocation` _capsulecomponent_3)))
  (bind (_returnvalue_x_7 _returnvalue_y_7) (`KismetMathLibrary.BreakVector` (`SceneComponent.K2_GetComponentLocation` (`self.Go to Left Start`))))
  (bind (_returnvalue_x_8 _returnvalue_y_8 _returnvalue_z_4) (`KismetMathLibrary.BreakVector` (`SceneComponent.K2_GetComponentLocation` _capsulecomponent_4)))
  (bind (_returnvalue_x_9 _returnvalue_y_9) (`KismetMathLibrary.BreakVector` (`SceneComponent.K2_GetComponentLocation` (`self.Go to Right End`))))
  (bind (_returnvalue_x_10 _returnvalue_y_10 _returnvalue_z_5) (`KismetMathLibrary.BreakVector` (`SceneComponent.K2_GetComponentLocation` _capsulecomponent_5)))
  ;[1 0 0.0652] Open Door Logic
  (if (== OtherActor (`.Character` (`/Game/Code/NaturalMovementV3/Blueprint/NMFunctionLibrary/BP_NMFunctionLibrary.NMCharacter`)))
    (`|ExecutionSequence`
      (:`then_0`
        (`self.Active Trace` (`self.varHold`) :!label _label
          (:`Out Left Door [true]`
            (`/Engine/EditorBlueprintResources/StandardMacros.DoOnce` false :!label _label_2
              (:`Completed`
                (bind (_direction _1) (`Timeline|Left Timeline` :!via `PlayFromStart`)
                  (:`Update`
                    (`|ExecutionSequence`
                      (:`then_0`
                        (`/Engine/EditorBlueprintResources/StandardMacros.DoOnce` false :!label _label_3
                          (:`Completed`
                            (`KismetSystemLibrary.MoveComponentTo` _capsulecomponent_4 (`KismetMathLibrary.MakeVector` _returnvalue_x_7 _returnvalue_y_7 _returnvalue_z_4) (`SceneComponent.RelativeRotation` _capsulecomponent_4) true true 0.4)
                            (`KismetSystemLibrary.MoveComponentTo` _capsulecomponent_3 (`KismetMathLibrary.MakeVector` _returnvalue_x_5 _returnvalue_y_5 _returnvalue_z_3) (`SceneComponent.RelativeRotation` _capsulecomponent_3) true true 2.0)
                            (`/Game/Code/NaturalMovementV3/Blueprint/NMFunctionLibrary/BP_NMFunctionLibrary.Enable Movement`)
                            (`SceneComponent.K2_SetRelativeRotation` :`self` (`self.SM_Door`))
                            (goto _label_3 :!via `Reset`))))
                      (:`then_1`
                        (`self.DoorRotation` _1 (struct :`Yaw` 90.0) 1.0))
                      (:`then_2`
                        (`/Game/Code/NaturalMovementV3/Blueprint/NMFunctionLibrary/BP_NMFunctionLibrary.Disable Movement`))))
                  (:`Finished`
                    (goto _label_2 :!via `Reset`))))))
          (:`thenOut Left Door [false]`
            (`/Engine/EditorBlueprintResources/StandardMacros.DoOnce` false :!label _label_4
              (:`Completed`
                (bind (_direction_2 _1_2) (`Timeline|Right Timeline` :!via `PlayFromStart`)
                  (:`Update`
                    (`|ExecutionSequence`
                      (:`then_0`
                        (`/Engine/EditorBlueprintResources/StandardMacros.DoOnce` false :!label _label_5
                          (:`Completed`
                            (`KismetSystemLibrary.MoveComponentTo` _capsulecomponent (`KismetMathLibrary.MakeVector` _returnvalue_x _returnvalue_y _returnvalue_z) (`SceneComponent.RelativeRotation` _capsulecomponent) true true 0.4)
                            (`KismetSystemLibrary.MoveComponentTo` _capsulecomponent_2 (`KismetMathLibrary.MakeVector` _returnvalue_x_3 _returnvalue_y_3 _returnvalue_z_2) (`SceneComponent.RelativeRotation` _capsulecomponent_2) true true 2.0)
                            (`/Game/Code/NaturalMovementV3/Blueprint/NMFunctionLibrary/BP_NMFunctionLibrary.Enable Movement`)
                            (`SceneComponent.K2_SetRelativeRotation` :`self` (`self.SM_Door`))
                            (goto _label_5 :!via `Reset`))))
                      (:`then_1`
                        (`self.DoorRotation` _1_2 (struct :`Yaw` -90.0) 1.0))
                      (:`then_2`
                        (`/Game/Code/NaturalMovementV3/Blueprint/NMFunctionLibrary/BP_NMFunctionLibrary.Disable Movement`))))
                  (:`Finished`
                    (goto _label_4 :!via `Reset`))))))))
      (:`then_1`
        ;;[1 0 0.0652] Door Kick
        (`self.CanDoorKickRight`
          (:`true`
            (if (and (`/Game/Code/NaturalMovementV3/Blueprint/NMFunctionLibrary/BP_NMFunctionLibrary.InState?` "NewEnumerator4") (not (`/Game/Code/NaturalMovementV3/Blueprint/NMFunctionLibrary/BP_NMFunctionLibrary.InAir?`)))
              (if (> (`/Game/Code/NaturalMovementV3/Blueprint/NMFunctionLibrary/BP_NMFunctionLibrary.NMVectorLenght`) 300.0)
                (set `/Game/Code/GameMain/LowPolyShooterPack/Core/Characters/BP_LPSP_PCH.varEnumMouseInput` "NewEnumerator0" (`.Character_LPSP` (`/Game/Code/NaturalMovementV3/Blueprint/NMFunctionLibrary/BP_NMFunctionLibrary.NMCharacter`)))
                (bind (_direction_3 _1_3) (`Timeline|Timeline_01` :!via `PlayFromStart`)
                  (:`Update`
                    (`|ExecutionSequence`
                      (:`then_0`
                        (`/Engine/EditorBlueprintResources/StandardMacros.DoOnce` false :!label _label_6
                          (:`Completed`
                            (`PlayerCameraManager.PlayCameraAnim` :`self` (`GameplayStatics.GetPlayerCameraManager` 0) :`Anim` "/Game/Code/NaturalMovementV3/Blueprint/Misc/CameraAnimations/CA_DoorKick_Right.CA_DoorKick_Right")
                            (`/Game/Code/NaturalMovementV3/Blueprint/NMFunctionLibrary/BP_NMFunctionLibrary.Disable Movement`)
                            (`|ExecutionSequence`
                              (:`then_0`
                                (`KismetSystemLibrary.MoveComponentTo` _capsulecomponent_5 (`KismetMathLibrary.MakeVector` _returnvalue_x_9 _returnvalue_y_9 _returnvalue_z_5) (`SceneComponent.K2_GetComponentRotation` _capsulecomponent_5) false false 0.7)
                                (if _isnmcharacter
                                  (`|ExecutionSequence`
                                    (:`then_0`
                                      (if (`/Game/Code/NaturalMovementV3/Blueprint/Character/BP_NMCharacter.varSprintKeyDown` _character_nm)
                                        (set `/Game/Code/NaturalMovementV3/Blueprint/Character/BP_NMCharacter.varEnumPlayerState` "NewEnumerator4" _character_nm)))
                                    (:`then_1`
                                      (`KismetSystemLibrary.Delay` 0.1)
                                      (`SceneComponent.K2_SetRelativeRotation` :`self` (`self.SM_Door`))))
                                  (else
                                    (`|ExecutionSequence`
                                      (:`then_0`
                                        (if (`/Game/Code/GameMain/LowPolyShooterPack/Core/Characters/BP_LPSP_PCH.Running` _character_lpsp)
                                          (set `/Game/Code/GameMain/LowPolyShooterPack/Core/Characters/BP_LPSP_PCH.varEnumPlayerState` "NewEnumerator4" _character_lpsp)))
                                      (:`then_1`
                                        (`KismetSystemLibrary.Delay` 0.1)
                                        (`SceneComponent.K2_SetRelativeRotation` :`self` (`self.SM_Door`)))))))
                              (:`then_1`
                                (`KismetSystemLibrary.Delay` 0.5)
                                (`/Game/Code/NaturalMovementV3/Blueprint/NMFunctionLibrary/BP_NMFunctionLibrary.Enable Movement`)
                                (set `/Game/Code/GameMain/LowPolyShooterPack/Core/Characters/BP_LPSP_PCH.varEnumMouseInput` "NewEnumerator1" (`.Character_LPSP` (`/Game/Code/NaturalMovementV3/Blueprint/NMFunctionLibrary/BP_NMFunctionLibrary.NMCharacter`))))))))
                      (:`then_2`
                        (`self.DoorRotation` _1_3 (struct :`Yaw` -90.0) 10.0))))
                  (:`Finished`
                    (goto _label_6 :!via `Reset`))))))))
      (:`then_2`
        (bind _aswbp_door_interact (`self.Widget`))
        (`/Game/Code/NaturalMovementV3/UI/Widgets/WBP_DoorInteract.Show Widget` _aswbp_door_interact)))))

(event `self.ActiveDoorTrace_2.OnComponentEndOverlap`
  (params (OverlappedComponent :type "PrimitiveComponent Object Reference") (OtherActor :type "Actor Object Reference") (OtherComp :type "PrimitiveComponent Object Reference") (OtherBodyIndex :type Integer))
  ;[1 0 0.0652] Open Door Logic
  (if (== OtherActor (`.Character` (`/Game/Code/NaturalMovementV3/Blueprint/NMFunctionLibrary/BP_NMFunctionLibrary.NMCharacter`)))
    (`|ExecutionSequence`
      (:`then_0`
        (goto _label :!via `End Overlap`))
      (:`then_1`
        (bind _aswbp_door_interact (`self.Widget`))
        (`/Game/Code/NaturalMovementV3/UI/Widgets/WBP_DoorInteract.Hide Widget` _aswbp_door_interact)))))

(event `self.ActiveDoorTrace_1.OnComponentBeginOverlap`
  (params (OverlappedComponent :type "PrimitiveComponent Object Reference") (OtherActor :type "Actor Object Reference") (OtherComp :type "PrimitiveComponent Object Reference") (OtherBodyIndex :type Integer) (bFromSweep :type Boolean) (SweepResult :type "HitResult Structure (by ref)"))
  (bind _capsulecomponent (`/Game/Code/NaturalMovementV3/Blueprint/NMFunctionLibrary/BP_NMFunctionLibrary.NMCapsuleComponent`))
  (bind (_character_nm _character_lpsp _camera _character _isnmcharacter) (`/Game/Code/NaturalMovementV3/Blueprint/NMFunctionLibrary/BP_NMFunctionLibrary.NMCharacter`))
  (bind (_returnvalue_x _returnvalue_y) (`KismetMathLibrary.BreakVector` (`SceneComponent.K2_GetComponentLocation` (`self.Go to Left End`))))
  (bind (_returnvalue_x_2 _returnvalue_y_2 _returnvalue_z) (`KismetMathLibrary.BreakVector` (`SceneComponent.K2_GetComponentLocation` _capsulecomponent)))
  ;[1 0 0.0652] Open Door Logic
  (if (== OtherActor (`.Character` (`/Game/Code/NaturalMovementV3/Blueprint/NMFunctionLibrary/BP_NMFunctionLibrary.NMCharacter`)))
    (`|ExecutionSequence`
      (:`then_0`
        (goto _label))
      (:`then_1`
        ;;[1 0 0.0652] Door Kick
        (`self.CanDoorKickLeft`
          (:`true`
            (if (and (`/Game/Code/NaturalMovementV3/Blueprint/NMFunctionLibrary/BP_NMFunctionLibrary.InState?` "NewEnumerator4") (not (`/Game/Code/NaturalMovementV3/Blueprint/NMFunctionLibrary/BP_NMFunctionLibrary.InAir?`)))
              (if (> (`/Game/Code/NaturalMovementV3/Blueprint/NMFunctionLibrary/BP_NMFunctionLibrary.NMVectorLenght`) 300.0)
                (set `/Game/Code/GameMain/LowPolyShooterPack/Core/Characters/BP_LPSP_PCH.varEnumMouseInput` "NewEnumerator0" (`.Character_LPSP` (`/Game/Code/NaturalMovementV3/Blueprint/NMFunctionLibrary/BP_NMFunctionLibrary.NMCharacter`)))
                (bind (_direction _1) (`Timeline|Run Left` :!via `PlayFromStart`)
                  (:`Update`
                    (`|ExecutionSequence`
                      (:`then_0`
                        (`/Engine/EditorBlueprintResources/StandardMacros.DoOnce` false :!label _label_7
                          (:`Completed`
                            (`PlayerCameraManager.PlayCameraAnim` :`self` (`GameplayStatics.GetPlayerCameraManager` 0) :`Anim` "/Game/Code/NaturalMovementV3/Blueprint/Misc/CameraAnimations/CA_DoorKick_Left.CA_DoorKick_Left")
                            (`/Game/Code/NaturalMovementV3/Blueprint/NMFunctionLibrary/BP_NMFunctionLibrary.Disable Movement`)
                            (`|ExecutionSequence`
                              (:`then_0`
                                (`KismetSystemLibrary.MoveComponentTo` _capsulecomponent (`KismetMathLibrary.MakeVector` _returnvalue_x _returnvalue_y _returnvalue_z) (`SceneComponent.K2_GetComponentRotation` _capsulecomponent) false false 0.7)
                                (if _isnmcharacter
                                  (`|ExecutionSequence`
                                    (:`then_0`
                                      (if (`/Game/Code/NaturalMovementV3/Blueprint/Character/BP_NMCharacter.varSprintKeyDown` _character_nm)
                                        (set `/Game/Code/NaturalMovementV3/Blueprint/Character/BP_NMCharacter.varEnumPlayerState` "NewEnumerator4" _character_nm)))
                                    (:`then_1`
                                      (`SceneComponent.K2_SetRelativeRotation` :`self` (`self.SM_Door`))))
                                  (else
                                    (`|ExecutionSequence`
                                      (:`then_0`
                                        (if (`/Game/Code/GameMain/LowPolyShooterPack/Core/Characters/BP_LPSP_PCH.Running` _character_lpsp)
                                          (set `/Game/Code/GameMain/LowPolyShooterPack/Core/Characters/BP_LPSP_PCH.varEnumPlayerState` "NewEnumerator4" _character_lpsp)))
                                      (:`then_1`
                                        (`SceneComponent.K2_SetRelativeRotation` :`self` (`self.SM_Door`)))))))
                              (:`then_1`
                                (`KismetSystemLibrary.Delay` 0.5)
                                (`/Game/Code/NaturalMovementV3/Blueprint/NMFunctionLibrary/BP_NMFunctionLibrary.Enable Movement`)
                                (set `/Game/Code/GameMain/LowPolyShooterPack/Core/Characters/BP_LPSP_PCH.varEnumMouseInput` "NewEnumerator1" (`.Character_LPSP` (`/Game/Code/NaturalMovementV3/Blueprint/NMFunctionLibrary/BP_NMFunctionLibrary.NMCharacter`))))))))
                      (:`then_2`
                        (`self.DoorRotation` _1 (struct :`Yaw` 90.0) 10.0))))
                  (:`Finished`
                    (goto _label_7 :!via `Reset`))))))))
      (:`then_2`
        (bind _aswbp_door_interact (`self.Widget`))
        (`/Game/Code/NaturalMovementV3/UI/Widgets/WBP_DoorInteract.Show Widget` _aswbp_door_interact)
        (set `self.varHold` 0.0)))))

(event `self.ActiveDoorTrace_1.OnComponentEndOverlap`
  (params (OverlappedComponent :type "PrimitiveComponent Object Reference") (OtherActor :type "Actor Object Reference") (OtherComp :type "PrimitiveComponent Object Reference") (OtherBodyIndex :type Integer))
  ;[1 0 0.0652] Open Door Logic
  (if (== OtherActor (`.Character` (`/Game/Code/NaturalMovementV3/Blueprint/NMFunctionLibrary/BP_NMFunctionLibrary.NMCharacter`)))
    (`|ExecutionSequence`
      (:`then_0`
        (goto _label :!via `End Overlap`))
      (:`then_1`
        (bind _aswbp_door_interact (`self.Widget`))
        (`/Game/Code/NaturalMovementV3/UI/Widgets/WBP_DoorInteract.Hide Widget` _aswbp_door_interact)
        (set `self.varHold` 0.0)))))

(event `InputAction|Interaction`
  (params (Key :type "Key Structure"))
  ;[1 0 0.0652] Open Door Logic
  (:`Pressed`
    (bind (_direction _holdtime) (`Timeline|Hold` :!via `PlayFromStart` :!label _label_8)
      (:`Update`
        (set `self.varHold` _holdtime)
        (`|ExecutionSequence`
          (:`then_0`
            (if (`/Game/Code/NaturalMovementV3/Blueprint/NMFunctionLibrary/BP_NMFunctionLibrary.InState?` "NewEnumerator1")
              (goto _label :!via `Key`)
              (else
                (set `self.varHold` 0.0))))
          (:`then_1`
            (bind _aswbp_door_interact (`self.Widget`))
            (`ProgressBar.SetPercent` (`/Game/Code/NaturalMovementV3/UI/Widgets/WBP_DoorInteract.ProgressBar_82` _aswbp_door_interact) (`self.varHold`)))))))
  (:`Released`
    (goto _label_8 :!via `Reverse`)))

(fn `ResetCameraLeft`
  (bind _returnvalue (`Pawn.GetControlRotation` (`.Character` (`/Game/Code/NaturalMovementV3/Blueprint/NMFunctionLibrary/BP_NMFunctionLibrary.NMCharacter`))))
  (bind (_returnvalue_roll _returnvalue_pitch _returnvalue_yaw) (`KismetMathLibrary.BreakRotator` (`SceneComponent.K2_GetComponentRotation` (`self.LeftStand`))))
  ;[1 0 0.0652] Reset Camera Left
  (`Controller.SetControlRotation` (`GameplayStatics.GetPlayerController` 0) (`KismetMathLibrary.RInterpTo` _returnvalue (`KismetMathLibrary.MakeRotator` (.roll _returnvalue) 0.0 _returnvalue_yaw) (`GameplayStatics.GetWorldDeltaSeconds`) 6.0)))

(fn `ResetCameraRight`
  (bind _rightstand (`self.RightStand`))
  (bind _returnvalue (`Pawn.GetControlRotation` (`.Character` (`/Game/Code/NaturalMovementV3/Blueprint/NMFunctionLibrary/BP_NMFunctionLibrary.NMCharacter`))))
  (bind (_returnvalue_roll _returnvalue_pitch _returnvalue_yaw) (`KismetMathLibrary.BreakRotator` (`SceneComponent.K2_GetComponentRotation` _rightstand)))
  ;[1 0 0.0652] Reset Camera Right
  (if (== (`SceneComponent.K2_GetComponentRotation` _rightstand) _returnvalue)
    (`KismetSystemLibrary.PrintString` "Hello")
    (else
      (`Controller.SetControlRotation` (`GameplayStatics.GetPlayerController` 0) (`KismetMathLibrary.RInterpTo` _returnvalue (`KismetMathLibrary.MakeRotator` (.roll _returnvalue) 0.0 _returnvalue_yaw) (`GameplayStatics.GetWorldDeltaSeconds`) 1.0)))))

(fn `UserConstructionScript`)