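; BP_GoalActor is a goal actor whose static mesh can orbit the actor's starting location.
; BeginPlay stores that location, and when UseAnimation is on, Tick advances a wrapping degree counter at OscillationRate.
; Sine and cosine of that angle, scaled by separate X and Y distances, move the mesh along a horizontal ellipse, with ChangeDir reversing the direction.
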(event `self.ReceiveBeginPlay`
  (set `self.InitialLocation` (`self.K2_GetActorLocation`)))

(event `self.ReceiveTick`
  (params (DeltaSeconds :type "Float (single-precision)"))
  (bind (_initiallocation_x _initiallocation_y _initiallocation_z) (`KismetMathLibrary.BreakVector` (`self.InitialLocation`)))
  (bind _returnvalue (* (`KismetSystemLibrary.MakeLiteralDouble` (`KismetMathLibrary.SelectFloat` 1.0 -1.0 (`self.Change Dir`))) (`self.degreesCounter`)))
  ;[1 1 1] Circular oscillator.
  (if (`self.UseAnimation`)
    (bind _output_get (set `self.degreesCounter` (+ (`self.degreesCounter`) (* DeltaSeconds (`self.Oscillation rate`)))))
    (if (> _output_get 359.0)
      (set `self.degreesCounter` 0.0))
    (`SceneComponent.K2_SetWorldLocation` (`self.StaticMesh1`) (`KismetMathLibrary.MakeVector` (+ (* (`KismetMathLibrary.DegSin` _returnvalue) (`self.X oscillation distance`)) _initiallocation_x) (+ (* (`KismetMathLibrary.DegCos` _returnvalue) (`self.Y oscillation distance`)) _initiallocation_y) _initiallocation_z) false false)))

(fn `UserConstructionScript`)