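; BP_RopeSwing is a rope swing actor whose Cone volume controls when the BP_LPSP_PCH player's RopeComponent can swing.
; Entering the cone clears the component's swing-force and tracer stop flags, increments its collision counter and stores the result.
; Leaving restores both flags and resets the counter only if it still matches the stored number, so exiting an earlier cone does not cancel a newer overlap.
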(event `self.Cone.OnComponentBeginOverlap`
  (params (OverlappedComponent :type "PrimitiveComponent Object Reference") (OtherActor :type "Actor Object Reference") (OtherComp :type "PrimitiveComponent Object Reference") (OtherBodyIndex :type Integer) (bFromSweep :type Boolean) (SweepResult :type "HitResult Structure (by ref)"))
  (bind _asbp_lpsp_pch (cast `/Game/Code/GameMain/LowPolyShooterPack/Core/Characters/BP_LPSP_PCH` OtherActor))
  (bind _rope_component (`/Game/Code/GameMain/LowPolyShooterPack/Core/Characters/BP_LPSP_PCH.Rope_Component` _asbp_lpsp_pch))
  (set `/Game/Code/RopeComponent/Rope_Component.stop swing force` false _rope_component)
  (set `/Game/Code/RopeComponent/Rope_Component.stop tracer` false _rope_component)
  (bind _result (`/Engine/EditorBlueprintResources/StandardMacros.IncrementInt` (`/Game/Code/RopeComponent/Rope_Component.CurrentCollsion` _rope_component))
    (:`  `
      (set `self.num` _result))))

(event `self.Cone.OnComponentEndOverlap`
  (params (OverlappedComponent :type "PrimitiveComponent Object Reference") (OtherActor :type "Actor Object Reference") (OtherComp :type "PrimitiveComponent Object Reference") (OtherBodyIndex :type Integer))
  (bind _asbp_lpsp_pch (cast `/Game/Code/GameMain/LowPolyShooterPack/Core/Characters/BP_LPSP_PCH` OtherActor))
  (if (== (`/Game/Code/RopeComponent/Rope_Component.CurrentCollsion` (`/Game/Code/GameMain/LowPolyShooterPack/Core/Characters/BP_LPSP_PCH.Rope_Component` (stale `self.Cone.OnComponentBeginOverlap` _asbp_lpsp_pch))) (`self.num`))
    (bind _rope_component (`/Game/Code/GameMain/LowPolyShooterPack/Core/Characters/BP_LPSP_PCH.Rope_Component` _asbp_lpsp_pch))
    (set `/Game/Code/RopeComponent/Rope_Component.stop swing force` true _rope_component)
    (set `/Game/Code/RopeComponent/Rope_Component.stop tracer` true _rope_component)
    (set `/Game/Code/RopeComponent/Rope_Component.CurrentCollsion` 0 _rope_component)))

(fn `UserConstructionScript`)