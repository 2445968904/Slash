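; Spline-following train actor that builds a row of static mesh carts and runs them around a looping track.
; The construction script spawns engines at both ends with cycling cart meshes between them and previews their placement.
; If TrainFunctional, a timeline at TrainSpeed drives MoveTrainLoop, restarting after TrainWaitingTime.
; MoveTrainLoop spaces carts by CartSpacing, wraps distances recursively via UpdateDistance and flips the first engine backwards.
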(event `self.ReceiveBeginPlay`
  (if (`self.TrainFunctional`)
    ;[1 1 1] Train Speed
    (`TimelineComponent.SetPlayRate` (`self.TrainMovement`) (`self.TrainSpeed`))
    ;[1 1 1] Train Movement Logic
    (bind (_direction _trainposition) (`Timeline|TrainMovement` :!via `PlayFromStart` :!label _label)
      (:`Update`
        (`self.MoveTrain_Loop` _trainposition))
      (:`Finished`
        (`KismetSystemLibrary.Delay` (`self.TrainWaitingTime`))
        (goto _label :!via `PlayFromStart`)))))

(event `self.ReceiveTick`
  (params (DeltaSeconds :type "Float (single-precision)"))
  (`parent.ReceiveTick` DeltaSeconds))

(fn `CreateTrain`
  (bind _cartnumber (`self.CartNumber`))
  ;[1 1 1] Choose Cart Mesh
  (for _index (range (`self.NumberOfCarts`))
    (if (>= (`self.CartNumber`) (- (`KismetArrayLibrary.Array_Length` (`self.CartMeshes`)) 1))
      (set `self.CartNumber` 0)
      (else
        (set `self.CartNumber` (+ 1 _cartnumber))))
    (`KismetSystemLibrary.PrintString` (`KismetStringLibrary.Conv_IntToString` _cartnumber))
    ;[1 1 1] Add Trains
    (bind _returnvalue (`AddComponent|NODE_AddStaticMeshComponent-0`))
    (`KismetArrayLibrary.Array_Add` (`self.TrainCarts`) _returnvalue)
    (if (== _index 0)
      (`StaticMeshComponent.SetStaticMesh` _returnvalue "/Game/BlockingStarterPack/Props/Vehicle/SM_Train_Engine1.SM_Train_Engine1")
      (elif (== _index (- (`self.NumberOfCarts`) 1))
        (`StaticMeshComponent.SetStaticMesh` _returnvalue "/Game/BlockingStarterPack/Props/Vehicle/SM_Train_Engine1.SM_Train_Engine1")
        (else
          (`StaticMeshComponent.SetStaticMesh` _returnvalue (`|GetArrayItem` (`self.CartMeshes`) (`self.CartNumber`))))))))

(fn `GetSplinePoint`
  (params (index :type Integer))
  (returns (Distance :type "Float (double-precision)"))
  (return 0.0))

(fn `MoveTrain`
  (params (TrainPosition :type "Float (double-precision)") (Reverse :type Boolean))
  (bind _spline (`self.Spline`))
  ;[1 1 1] Move Carts
  (for (_array_element _array_index) (`self.TrainCarts`)
    (`/Engine/EditorBlueprintResources/StandardMacros.IsValid` _array_element
      (:`Is Valid`
        (bind _returnvalue (+ (`KismetMathLibrary.Lerp` 0.0 (`SplineComponent.GetSplineLength` _spline) TrainPosition) (* _array_index (* (`KismetMathLibrary.SelectFloat` -1.0 1.0 (`self.reverse`)) (`self.CartSpacing`)))))
        (`SceneComponent.K2_SetRelativeLocationAndRotation` _array_element (`KismetMathLibrary.MakeVector` (.x (`SplineComponent.GetLocationAtDistanceAlongSpline` _spline _returnvalue "Local")) (.y (`SplineComponent.GetLocationAtDistanceAlongSpline` _spline _returnvalue "Local")) (+ (.z (`SplineComponent.GetLocationAtDistanceAlongSpline` _spline _returnvalue "Local")) (`self.TrainDeviation`))) (`KismetMathLibrary.MakeRotator` (.roll (`SplineComponent.GetRotationAtDistanceAlongSpline` _spline _returnvalue "Local")) (.pitch (`SplineComponent.GetRotationAtDistanceAlongSpline` _spline _returnvalue "Local")) (.yaw (`SplineComponent.GetRotationAtDistanceAlongSpline` _spline _returnvalue "Local"))) false false)))))

(fn `MoveTrain_Loop`
  (params (TrainPosition :type "Float (double-precision)") (Reverse :type Boolean))
  (bind _spline (`self.Spline`))
  ;[1 1 1] Move Carts
  (for (_array_element _array_index) (`self.TrainCarts`)
    (`/Engine/EditorBlueprintResources/StandardMacros.IsValid` _array_element
      (:`Is Valid`
        (bind _out (`self.UpdateDistance` (+ (`KismetMathLibrary.Lerp` 0.0 (`SplineComponent.GetSplineLength` _spline) TrainPosition) (* _array_index (`self.CartSpacing`)))))
        (`SceneComponent.K2_SetRelativeLocationAndRotation` _array_element (`KismetMathLibrary.MakeVector` (.x (`SplineComponent.GetLocationAtDistanceAlongSpline` _spline _out "Local")) (.y (`SplineComponent.GetLocationAtDistanceAlongSpline` _spline _out "Local")) (+ (.z (`SplineComponent.GetLocationAtDistanceAlongSpline` _spline _out "Local")) (`self.TrainDeviation`))) (`KismetMathLibrary.MakeRotator` (.roll (`SplineComponent.GetRotationAtDistanceAlongSpline` _spline _out "Local")) (.pitch (`SplineComponent.GetRotationAtDistanceAlongSpline` _spline _out "Local")) (.yaw (`SplineComponent.GetRotationAtDistanceAlongSpline` _spline _out "Local"))) false false)
        (`|ExecutionSequence`
          (:`then_0`
            (`PrimitiveComponent.SetCastShadow` _array_element false))
          (:`then_1`
            (if (== _array_index 0)
              (bind (_relativerotation_roll _relativerotation_pitch _relativerotation_yaw) (`KismetMathLibrary.BreakRotator` (`SceneComponent.RelativeRotation` _array_element)))
              (`SceneComponent.K2_SetRelativeRotation` _array_element (`KismetMathLibrary.MakeRotator` _relativerotation_roll (* _relativerotation_pitch -1.0) (+ _relativerotation_yaw 180.0)) false false))))))))

(fn `UpdateDistance`
  (params (Distance :type "Float (double-precision)"))
  (returns (out :type "Float (double-precision)"))
  (bind _returnvalue (`SplineComponent.GetSplineLength` (`self.Spline`)))
  (if (> Distance _returnvalue)
    (return (`self.UpdateDistance` (- Distance _returnvalue)))
    (else
      (return Distance))))

(fn `UserConstructionScript`
  (`parent.UserConstructionScript`)
  (`self.CreateTrain`)
  (`self.MoveTrain_Loop` (`self.TrainPosition`)))