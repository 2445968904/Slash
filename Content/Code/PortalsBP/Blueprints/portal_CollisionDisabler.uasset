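; Portal helper actor that disables collision between a moving component and the blocking walls behind a portal and its target portal.
; On BeginPlay, physics-simulating primitives are linked to each valid wall through two physics constraints, using constraints as a per-pair collision filter.
; Capsule components instead ignore each wall's owning actor when moving.
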(event `self.ReceiveBeginPlay`
  (bind _portal (`self.Portal`))
  (bind _portal_2 (`self.Portal`))
  (bind _moveableactor (`self.MoveableActor`))
  (bind _blockingwall (`/Game/Code/PortalsBP/Blueprints/PortalBP.BlockingWall` _portal))
  (bind _blockingwall_2 (`/Game/Code/PortalsBP/Blueprints/PortalBP.BlockingWall` _portal_2))
  (bind _blockingwall_3 (`/Game/Code/PortalsBP/Blueprints/PortalBP.BlockingWall` (`/Game/Code/PortalsBP/Blueprints/PortalBP.TargetPortal` _portal_2)))
  (bind _blockingwall_4 (`/Game/Code/PortalsBP/Blueprints/PortalBP.BlockingWall` (`/Game/Code/PortalsBP/Blueprints/PortalBP.TargetPortal` _portal)))
  (`|ExecutionSequence`
    (:`then_0`
      (bind `_as基元组件` (cast `PrimitiveComponent` _moveableactor))
      ;[1 1 1] disable collision for primative
      (if (`SceneComponent.IsSimulatingPhysics` `_as基元组件` "None")
        (`|ExecutionSequence`
          (:`then_0`
            (`/Engine/EditorBlueprintResources/StandardMacros.IsValid` _blockingwall_4
              (:`Is Valid`
                (`PhysicsConstraintComponent.SetConstrainedComponents` (`self.PhysicsConstraint`) `_as基元组件` "None" _blockingwall_4 "None"))))
          (:`then_1`
            (`/Engine/EditorBlueprintResources/StandardMacros.IsValid` _blockingwall
              (:`Is Valid`
                (`PhysicsConstraintComponent.SetConstrainedComponents` (`self.PhysicsConstraint1`) `_as基元组件` "None" _blockingwall "None")))))))
    (:`then_1`
      ;[1 1 1] disable collision for capsule
      (bind `_as胶囊体碰撞` (cast `CapsuleComponent` _moveableactor))
      (`|ExecutionSequence`
        (:`then_0`
          (`/Engine/EditorBlueprintResources/StandardMacros.IsValid` _blockingwall_3
            (:`Is Valid`
              (`PrimitiveComponent.IgnoreActorWhenMoving` `_as胶囊体碰撞` (`ActorComponent.GetOwner` _blockingwall_3) true))))
        (:`then_1`
          (`/Engine/EditorBlueprintResources/StandardMacros.IsValid` _blockingwall_2
            (:`Is Valid`
              (`PrimitiveComponent.IgnoreActorWhenMoving` `_as胶囊体碰撞` (`ActorComponent.GetOwner` _blockingwall_2) true))))))))

(fn `UserConstructionScript`)