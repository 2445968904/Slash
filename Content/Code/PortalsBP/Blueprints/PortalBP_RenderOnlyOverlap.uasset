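; A portal Blueprint variant that, by its name, renders only on overlap, with rendering disabled shortly after play begins.
; On BeginPlay it runs the parent logic, casts the RenderCheck child actor to PortalrenderEnabler, waits briefly, gives it a reference to itself and clears RenderEnabled.
; Tick and construction only call the parent; the code that re-enables rendering is outside this Blueprint.
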(event `self.ReceiveBeginPlay`
  (`parent.ReceiveBeginPlay`)
  (bind _asportalrender_enabler (cast `/Game/Code/PortalsBP/Blueprints/PortalrenderEnabler` (`ChildActorComponent.ChildActor` (`self.RenderCheck`))))
  (`KismetSystemLibrary.Delay` 0.2)
  (set `/Game/Code/PortalsBP/Blueprints/PortalrenderEnabler.PortalRef` self _asportalrender_enabler)
  (set `self.RenderEnabled` false))

(event `self.ReceiveTick`
  (params (DeltaSeconds :type "Float (single-precision)"))
  (`parent.ReceiveTick` DeltaSeconds))

(fn `UserConstructionScript`
  (`parent.UserConstructionScript`))