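; BP_Build_Wall is a blockout building actor that generates a box mesh, named as a wall, sized by BoxSize.
; The construction script calls BlockoutRoundVector on BoxSize with RoundSize, then adds the box and calls BlockoutSetMaterial.
; AddBlockoutBox creates a static mesh component at the actor origin using BlockoutBoxMesh, scaled to BoxSize divided by 100.
; The event graph holds only disabled stub events, so it has no runtime logic.
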(fn `AddBlockoutBox`
  (bind _returnvalue (`AddComponent|NODE_AddStaticMeshComponent-0` :`RelativeTransform` (`KismetMathLibrary.MakeTransform` (0.0 0.0 0.0) (struct) (* (`self.BoxSize`) (/ 1.0 100.0)))))
  (`StaticMeshComponent.SetStaticMesh` _returnvalue (`self.BlockoutBoxMesh`)))

(fn `UserConstructionScript`
  (`/BlockoutToolsPlugin/Blueprints/Utility/BlockoutToolsFunctions.BlockoutRoundVector` (`self.bRoundSize`) (`self.BoxSize`))
  (`self.AddBlockoutBox`)
  (`self.BlockoutSetMaterial`))