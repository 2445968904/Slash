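; Toon point light actor for an anime toon-shading setup, working through a Scene object that manages mesh lighting.
; The construction script tells the Scene to update lighting on all meshes and tints the billboard mesh with LightColor through a dynamic material instance.
; ChangeScene moves the light's registration from the old Scene's LightsOnScene list to the new one, without itself triggering a lighting update.
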(fn `ChangeScene`
  (params (NewScene :type "/Game/Shader/AnimeToonShading/Blueprints/BP_ToonScene Object Reference"))
  (bind _newscene (`local.NewScene`))
  (bind _scene (`self.Scene`))
  (if (!= _scene NewScene)
    (if (`KismetSystemLibrary.IsValid` _scene)
      (`KismetArrayLibrary.Array_RemoveItem` (`/Game/Shader/AnimeToonShading/Blueprints/BP_ToonScene.Lights on scene` _scene) self))
    (set `self.Scene` _newscene)
    (`KismetArrayLibrary.Array_AddUnique` (`/Game/Shader/AnimeToonShading/Blueprints/BP_ToonScene.Lights on scene` _newscene) self)))

(fn `UserConstructionScript`
  (`/Game/Shader/AnimeToonShading/Blueprints/BP_ToonScene.UpdateAllMeshesLighting` (`self.Scene`) true)
  (bind _returnvalue (`PrimitiveComponent.CreateDynamicMaterialInstance` (`self.BillboardMesh`) 0 null "None"))
  (`MaterialInstanceDynamic.SetVectorParameterValue` _returnvalue "BaseColor" (`self.LightColor`)))