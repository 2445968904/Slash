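; BP_ToonDirectionalLight is an actor that supplies directional light and ambient data to the toon shading materials.
; ApplySettings writes the light color, the Front component's world forward vector and the skylight ambient into the MP_ToonShading Material Parameter Collection.
; It runs from the construction script, on BeginPlay, and on ticks paced by TickInterval, with a negative interval skipping the tick updates.
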(event `self.ReceiveBeginPlay`
  (`self.SetActorTickInterval` (`self.TickInterval`))
  (`self.ApplySettings`))

(event `self.ReceiveTick`
  (params (DeltaSeconds :type "Float (single-precision)"))
  (if (>= (`self.TickInterval`) 0.0)
    (`self.ApplySettings`)))

(fn `ApplySettings`
  (`KismetMaterialLibrary.SetVectorParameterValue` "/Game/Shader/AnimeToonShading/Materials/MP_ToonShading.MP_ToonShading" "DirectionalColor" (`self.LightColor`))
  (`KismetMaterialLibrary.SetVectorParameterValue` "/Game/Shader/AnimeToonShading/Materials/MP_ToonShading.MP_ToonShading" "DirectionalDirection" (`KismetMathLibrary.Conv_VectorToLinearColor` (`KismetMathLibrary.GetForwardVector` (`SceneComponent.K2_GetComponentRotation` (`self.Front`)))))
  (`KismetMaterialLibrary.SetVectorParameterValue` "/Game/Shader/AnimeToonShading/Materials/MP_ToonShading.MP_ToonShading" "SkylightAmbient" (`self.SkylightAmbient`)))

(fn `UserConstructionScript`
  (`self.ApplySettings`))