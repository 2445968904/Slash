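; BP_ToonStatic is a static mesh actor that applies toon shading and a colored shell through its BPToonComponent.
; The construction script passes the mesh and scene to ApplyShading and initializes the shell, which BeginPlay initializes again.
; The IToonShading interface event reapplies shading at runtime with a supplied scene, storing it on the actor.
; CreateShell is an empty stub.
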(event `/Game/Shader/AnimeToonShading/Blueprints/BI_ToonShading.IToonShading`
  (params (Construction :type Boolean) (Scane :type "/Game/Shader/AnimeToonShading/Blueprints/BP_ToonScene Object Reference"))
  (`self.ToonShading` false Scane))

(event `self.ReceiveBeginPlay`
  (`/Game/Shader/AnimeToonShading/Blueprints/BP_ToonComponent.InitStaticShell` (`self.BP_ToonComponent`) (`self.Shell`) (`self.ShellColor`)))

(fn `CreateShell`
  (locals (Triangles :type "Array of Integer")))

(fn `ToonShading`
  (params (Construction :type Boolean) (Scene :type "/Game/Shader/AnimeToonShading/Blueprints/BP_ToonScene Object Reference"))
  (bind _output_get (set `self.Scene` Scene))
  (`/Game/Shader/AnimeToonShading/Blueprints/BP_ToonComponent.ApplyShading` (`self.BP_ToonComponent`) Construction (`self.StaticMesh`) _output_get))

(fn `UserConstructionScript`
  (`self.ToonShading` true (`self.Scene`))
  (`/Game/Shader/AnimeToonShading/Blueprints/BP_ToonComponent.InitStaticShell` (`self.BP_ToonComponent`) (`self.Shell`) (`self.ShellColor`)))