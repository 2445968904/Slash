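; BP_ToonComponent is a component that applies toon lighting and colored shells to meshes.
; ApplyShading optionally creates dynamic materials, then passes the mesh and a location chosen by PositioningMode to the scene actor's ApplyMeshLighting.
; Shell setup assigns dynamic shell materials, binding skeletal shells to the source's pose via master pose.
; Shell color alpha doubles as shell width.
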(fn `ApplyShading`
  (params (Construction :type Boolean :default false) (Mesh :type "MeshComponent Object Reference") (ActorScene :type "/Game/Shader/AnimeToonShading/Blueprints/BP_ToonScene Object Reference"))
  (`/Engine/EditorBlueprintResources/StandardMacros.IsValid` ActorScene
    (:`Is Valid`
      (`/Engine/EditorBlueprintResources/StandardMacros.IsValid` Mesh
        (:`Is Valid`
          (if (`local.Construction`)
            (`self.CreateMaterials` (`local.Mesh`)))
          (switch `/Game/Shader/AnimeToonShading/Blueprints/PositioningMode` (`self.PositioningMode`)
            (:`NewEnumerator1`
              (`/Game/Shader/AnimeToonShading/Blueprints/BP_ToonScene.ApplyMeshLighting` (`local.ActorScene`) (`local.Mesh`) (`self.K2_GetComponentLocation`)))
            (:`NewEnumerator0`
              (`/Game/Shader/AnimeToonShading/Blueprints/BP_ToonScene.ApplyMeshLighting` (`local.ActorScene`) (`local.Mesh`) (`self.K2_GetComponentLocation` (`local.Mesh`))))
            (:`NewEnumerator2`
              (`/Game/Shader/AnimeToonShading/Blueprints/BP_ToonScene.ApplyMeshLighting` (`local.ActorScene`) (`local.Mesh`) (`KismetSystemLibrary.GetComponentBounds` (`local.Mesh`))))
            (:`NewEnumerator3`
              (`/Game/Shader/AnimeToonShading/Blueprints/BP_ToonScene.ApplyMeshLighting` (`local.ActorScene`) (`local.Mesh`) (`Actor.K2_GetActorLocation` (`self.GetOwner`))))))))))

(fn `CreateMaterials`
  (params (Mesh :type "MeshComponent Object Reference"))
  (for _ (range (+ (`PrimitiveComponent.GetNumMaterials` Mesh) 1))
    (`PrimitiveComponent.CreateDynamicMaterialInstance` Mesh 0 null "None")))

(fn `InitSkeletalShell`
  (params (Source :type "SkeletalMeshComponent Object Reference") (Shell :type "SkeletalMeshComponent Object Reference") (Color :type "LinearColor Structure"))
  (`SkinnedMeshComponent.SetLeaderPoseComponent` Shell Source false)
  (for _index (range (+ (`PrimitiveComponent.GetNumMaterials` Shell) 1))
    (`PrimitiveComponent.CreateDynamicMaterialInstance` Shell _index "/Game/Shader/AnimeToonShading/Materials/MI_ToonShadingShell.MI_ToonShadingShell" "None"))
  (`self.SetShellColor` Shell Color))

(fn `InitStaticShell`
  (params (Shell :type "StaticMeshComponent Object Reference") (Color :type "LinearColor Structure"))
  (bind _shell (`local.Shell`))
  (for _index (range (+ (`PrimitiveComponent.GetNumMaterials` Shell) 1))
    (bind _returnvalue (`PrimitiveComponent.CreateDynamicMaterialInstance` _shell _index "/Game/Shader/AnimeToonShading/Materials/MI_ToonShadingShell.MI_ToonShadingShell" "None"))
    ;[1 1 1] Editor preview
    (`MaterialInstanceDynamic.SetVectorParameterValue` _returnvalue "ShellColor" Color)
    (`MaterialInstanceDynamic.SetScalarParameterValue` _returnvalue "ShellWidth" (`.A` (break `LinearColor` Color))))
  (`self.SetShellColor` _shell Color))

(fn `SetShellColor`
  (params (Mesh :type "MeshComponent Object Reference") (ShellColor :type "LinearColor Structure"))
  (`MeshComponent.SetScalarParameterValueOnMaterials` Mesh "ShellWidth" (`.A` (break `LinearColor` ShellColor)))
  (`MeshComponent.SetVectorParameterValueOnMaterials` Mesh "ShellColor" (`KismetMathLibrary.Conv_LinearColorToVector` ShellColor)))